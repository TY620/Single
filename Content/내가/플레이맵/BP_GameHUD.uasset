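; BP_GameHUD is the game HUD Blueprint that puts the UW_GameWidget interface on screen.
; BeginPlay creates the widget, stores it as HUDWidget and adds it to the viewport.
; UpdateGold forwards a gold total to the widget's SetGold.
; A disconnected chain, which never runs, would bind to BP_PlayerState's CollectGold dispatcher and push the initial TotalGold through UpdateGold.
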(event `self.ReceiveBeginPlay`
  (bind _returnvalue (`|CreateWidget` "/Game/내가/위젯/UW_GameWidget.UW_GameWidget_C"))
  (bind _output_get (set `self.HUDWidget` _returnvalue))
  (`UserWidget.AddToViewport` _output_get 0))

(fn `UpdateGold`
  (params (TotalGold :type "Float (double-precision)"))
  (`/Game/내가/위젯/UW_GameWidget.SetGold` (`self.HUDWidget`) TotalGold))

(fn `UserConstructionScript`)