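; BP_BlinkFloor is a one-shot floor tile that vanishes shortly after the player character steps on it.
; A Box overlap filtered to BP_ThirdPersonCharacter turns the Cube green, then red as a warning after a short delay.
; After a second, shorter delay, the Cube is hidden and its collision is disabled rather than the actor being destroyed.
; Nothing restores the floor afterward.
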(event `self.Box.OnComponentBeginOverlap`
  (params (OverlappedComponent :type "PrimitiveComponent Object Reference") (OtherActor :type "Actor Object Reference") (OtherComp :type "PrimitiveComponent Object Reference") (OtherBodyIndex :type Integer) (bFromSweep :type Boolean) (SweepResult :type "HitResult Structure (by ref)"))
  (cast `/Game/ThirdPerson/Blueprints/BP_ThirdPersonCharacter` OtherActor)
  (`PrimitiveComponent.SetMaterial` (`self.Cube`) 0 "/AnimationSharing/AnimSharingGreen.AnimSharingGreen")
  (`KismetSystemLibrary.Delay` 1.0)
  (`PrimitiveComponent.SetMaterial` (`self.Cube`) 0 "/AnimationSharing/AnimSharingRed.AnimSharingRed")
  (`KismetSystemLibrary.Delay` 0.5)
  (`SceneComponent.SetVisibility` (`self.Cube`) false false)
  (`PrimitiveComponent.SetCollisionEnabled` (`self.Cube`) "NoCollision"))

(fn `UserConstructionScript`)