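; BP_PushFloor is a floor trap that briefly rotates and pushes the player character.
; Any overlap with its Box snaps the Cube to a rotated pose, then snaps it back after a short delay.
; When the Cube hits a BP_ThirdPersonCharacter, it applies a scaled-down hit normal impulse to that character's movement component.
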(event `self.Box.OnComponentHit`
  (params (HitComponent :type "PrimitiveComponent Object Reference") (OtherActor :type "Actor Object Reference") (OtherComp :type "PrimitiveComponent Object Reference") (NormalImpulse :type "Vector Structure") (Hit :type "HitResult Structure (by ref)")))

(event `self.Cube.OnComponentHit`
  (params (HitComponent :type "PrimitiveComponent Object Reference") (OtherActor :type "Actor Object Reference") (OtherComp :type "PrimitiveComponent Object Reference") (NormalImpulse :type "Vector Structure") (Hit :type "HitResult Structure (by ref)"))
  (bind _asbp_third_person_character (cast `/Game/ThirdPerson/Blueprints/BP_ThirdPersonCharacter` OtherActor))
  (`CharacterMovementComponent.AddImpulse` (`Character.CharacterMovement` _asbp_third_person_character) (* NormalImpulse 0.2) false)
  (if (not true)
    (`KismetSystemLibrary.PrintString` "Hello")))

(event `self.Box.OnComponentBeginOverlap`
  (params (OverlappedComponent :type "PrimitiveComponent Object Reference") (OtherActor :type "Actor Object Reference") (OtherComp :type "PrimitiveComponent Object Reference") (OtherBodyIndex :type Integer) (bFromSweep :type Boolean) (SweepResult :type "HitResult Structure (by ref)"))
  (`SceneComponent.K2_SetRelativeRotation` (`self.Cube`) (struct :`Pitch` 30.0) false false)
  (`KismetSystemLibrary.Delay` 0.8)
  (`SceneComponent.K2_SetRelativeRotation` :`self` (`self.Cube`)))

(fn `UserConstructionScript`)