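; BP_PushFloor is a floor trap that launches the player character when stepped on.
; Box overlap by any actor snaps the Cube to a rotated pose, then a cast filters for BP_ThirdPersonCharacter.
; The character receives a strong movement impulse along the rotated Cube's up vector.
; The Cube resets after a short delay only when the cast succeeds, so other actors leave it rotated.
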(event `self.Box.OnComponentBeginOverlap`
  (params (OverlappedComponent :type "PrimitiveComponent Object Reference") (OtherActor :type "Actor Object Reference") (OtherComp :type "PrimitiveComponent Object Reference") (OtherBodyIndex :type Integer) (bFromSweep :type Boolean) (SweepResult :type "HitResult Structure (by ref)"))
  (`SceneComponent.K2_SetRelativeRotation` (`self.Cube`) (struct :`Pitch` 40.0) false false)
  (bind _asbp_third_person_character (cast `/Game/ThirdPerson/Blueprints/BP_ThirdPersonCharacter` OtherActor))
  (`CharacterMovementComponent.AddImpulse` (`Character.CharacterMovement` _asbp_third_person_character) (* (`SceneComponent.GetUpVector` (`self.Cube`)) 80000.0) false)
  (`KismetSystemLibrary.Delay` 0.8)
  (`SceneComponent.K2_SetRelativeRotation` :`self` (`self.Cube`)))

(fn `UserConstructionScript`)