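; BP_Arrow is a physics-driven arrow projectile, filed under ArrowTrap, that damages the third-person player character.
; On BeginPlay it launches the Arrow component with a forward impulse, then destroys itself after a short delay.
; Component hits apply damage only to BP_ThirdPersonCharacter and do not destroy the arrow.
; Every tick it aligns the component's Z axis with its linear velocity, so the arrow points along its flight path.
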(event `self.ReceiveBeginPlay`
  (`PrimitiveComponent.AddImpulse` (`self.Arrow`) (* (`self.GetActorForwardVector`) 5000.0) "None" false)
  (`KismetSystemLibrary.Delay` 1.5)
  (`self.K2_DestroyActor`))

(event `self.Arrow.OnComponentHit`
  (params (HitComponent :type "PrimitiveComponent Object Reference") (OtherActor :type "Actor Object Reference") (OtherComp :type "PrimitiveComponent Object Reference") (NormalImpulse :type "Vector Structure") (Hit :type "HitResult Structure (by ref)"))
  (bind _asbp_third_person_character (cast `/Game/ThirdPerson/Blueprints/BP_ThirdPersonCharacter` OtherActor))
  (`GameplayStatics.ApplyDamage` _asbp_third_person_character 1.0))

(event `self.ReceiveTick`
  (params (DeltaSeconds :type "Float (single-precision)"))
  ;[1 1 1] 운동방향(Z)으로 회전 값 지정
  (bind _returnvalue (`PrimitiveComponent.GetPhysicsLinearVelocity` (`self.Arrow`) "None"))
  (`SceneComponent.K2_SetWorldRotation` (`self.Arrow`) (`KismetMathLibrary.MakeRotFromZ` _returnvalue) false false))

(fn `UserConstructionScript`)